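; Bp_Monster is a simple monster actor for a Dark Souls-style exercise that faces the player and can take damage.
; Every tick it sets its static mesh's yaw to look at player 0's character mesh, with pitch and roll fixed at zero.
; The DMG event prints a hit message and subtracts damage from PV.
; Tick destroys the actor only when PV equals exactly zero.
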(event `self.ReceiveTick`
  (params (DeltaSeconds :type "Float (single-precision)"))
  (bind (_returnvalue_roll _returnvalue_pitch _returnvalue_yaw) (`KismetMathLibrary.BreakRotator` (`KismetMathLibrary.FindLookAtRotation` (`SceneComponent.K2_GetComponentLocation` (`self.StaticMeshComponent0`)) (`SceneComponent.K2_GetComponentLocation` (`Character.Mesh` (`GameplayStatics.GetPlayerCharacter` 0))))))
  ;[1 1 1] desolé c'est shlag
  (`SceneComponent.K2_SetWorldRotation` (`self.StaticMeshComponent0`) (`KismetMathLibrary.MakeRotator` 0.0 0.0 _returnvalue_yaw) false false)
  (if (== (`self.PV`) 0.0)
    (`self.K2_DestroyActor`)))

(event `/Game/Devoir_remi/Dark_Souls/BPI/BPI_Combat.DMG`
  (params (Dmg :type "Float (double-precision)"))
  ;[1 1 1] recoit des dmgs
  (`KismetSystemLibrary.PrintString` "AIe")
  (set `self.PV` (- (`self.PV`) Dmg)))

(fn `UserConstructionScript`)