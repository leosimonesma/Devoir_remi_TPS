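; Melee monster enemy that turns to face the player, attacks at close range, and takes damage until it dies.
; Tick drives everything: it shows the monster's UI widget near the player, loops the attack montage in range, and plays a death montage before destroying the actor.
; Attack montage notifies open a damage window in which Box1 overlaps send damage, once per overlap.
; Incoming damage lowers PV and refreshes the widget.
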(event `self.ReceiveBeginPlay`
  ;[1 1 1] set UI
  (bind _returnvalue (`|CreateWidget` "/Game/Devoir_remi/Dark_Souls/UI/UI_Monstre.UI_Monstre_C"))
  (set `self.Monster_UI` _returnvalue)
  (`KismetSystemLibrary.PrintString` (`KismetStringLibrary.Conv_DoubleToString` (`self.PV`))))

(event `self.ReceiveTick`
  (params (DeltaSeconds :type "Float (single-precision)"))
  (bind (_returnvalue_roll _returnvalue_pitch _returnvalue_yaw) (`KismetMathLibrary.BreakRotator` (`KismetMathLibrary.FindLookAtRotation` (`SceneComponent.K2_GetComponentLocation` (`self.SkeletalMesh`)) (`SceneComponent.K2_GetComponentLocation` (`Character.Mesh` (`GameplayStatics.GetPlayerCharacter` 0))))))
  ;[1 1 1] desolé c'est shlag
  (if (<= (`self.GetDistanceTo` (`GameplayStatics.GetPlayerCharacter` 0)) 700.0)
    (`UserWidget.AddToViewport` (`self.Monster_UI`) 0)
    (else
      (`Widget.RemoveFromParent` (`self.Monster_UI`))))
  (if (<= (`self.PV`) 0.0)
    (`/Engine/EditorBlueprintResources/StandardMacros.DoOnce` false
      (:`Completed`
        (`|PlayMontage` (`self.SkeletalMesh`) "/Game/Devoir_remi/Dark_Souls/Anim/Monster/Montage_Death.Montage_Death"
          (:`OnNotifyEnd`
            (`self.K2_DestroyActor`)))))
    (else
      (`SceneComponent.K2_SetWorldRotation` (`self.SkeletalMesh`) (`KismetMathLibrary.MakeRotator` 0.0 0.0 (+ _returnvalue_yaw -90.0)) false false)
      (if (<= (`self.GetDistanceTo` (`GameplayStatics.GetPlayerCharacter` 0)) 500.0)
        (`/Engine/EditorBlueprintResources/StandardMacros.DoOnce` false :!label _label
          (:`Completed`
            (`|PlayMontage` (`self.SkeletalMesh`) "/Game/Devoir_remi/Dark_Souls/Anim/Monster/Attack_montage.Attack_montage"
              (:`OnCompleted`
                (goto _label :!via `Reset`))
              (:`OnNotifyBegin`
                (set `self.Do_DMG` true))
              (:`OnNotifyEnd`
                (set `self.Do_DMG` false)))))))))

(event `/Game/Devoir_remi/Dark_Souls/BPI/BPI_Combat.DMG_To_Monster`
  (params (Dmg :type "Float (double-precision)"))
  ;[1 1 1] recoit des dmgs
  (bind _output_get (set `self.PV` (- (`self.PV`) Dmg)))
  (`KismetSystemLibrary.PrintString` (`KismetStringLibrary.Conv_DoubleToString` _output_get))
  (message `/Game/Devoir_remi/Dark_Souls/BPI/BPI_Combat.Refresh_PV` (`self.Monster_UI`) _output_get))

(event `self.Box1.OnComponentBeginOverlap`
  (params (OverlappedComponent :type "PrimitiveComponent Object Reference") (OtherActor :type "Actor Object Reference") (OtherComp :type "PrimitiveComponent Object Reference") (OtherBodyIndex :type Integer) (bFromSweep :type Boolean) (SweepResult :type "HitResult Structure (by ref)"))
  ;[1 1 1] DMG
  (if (`self.Do_DMG`)
    (`/Engine/EditorBlueprintResources/StandardMacros.DoOnce` false :!label _label_2
      (:`Completed`
        (message `/Game/Devoir_remi/Dark_Souls/BPI/BPI_Combat.DMG_To_Player` OtherActor (`self.Monster_DMG`))))))

(event `self.Box1.OnComponentEndOverlap`
  (params (OverlappedComponent :type "PrimitiveComponent Object Reference") (OtherActor :type "Actor Object Reference") (OtherComp :type "PrimitiveComponent Object Reference") (OtherBodyIndex :type Integer))
  ;[1 1 1] DMG
  (goto _label_2 :!via `Reset`))

(fn `UserConstructionScript`)