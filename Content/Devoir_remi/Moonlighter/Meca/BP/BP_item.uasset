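; Interactable item actor that shows proximity icons to the player and can be inspected.
; Outer and inner collision spheres toggle their matching interaction icons as the player enters or leaves.
; On Interaction, if Inspect is set, it spawns a BP_inspectable and passes it the interactor, mesh, name, description, rotation and scale.
; The construction script applies mesh, scale, sphere radii and debug sphere visibility; the icon-location step is unconnected.
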(event `self.Outer_Sphere_Collision.OnComponentBeginOverlap`
  (params (OverlappedComponent :type "PrimitiveComponent Object Reference") (OtherActor :type "Actor Object Reference") (OtherComp :type "PrimitiveComponent Object Reference") (OtherBodyIndex :type Integer) (bFromSweep :type Boolean) (SweepResult :type "HitResult Structure (by ref)"))
  ;[1 1 1] Interaction icon visibility
  (if (== OtherActor (`GameplayStatics.GetPlayerCharacter` 0))
    (`SceneComponent.SetVisibility` (`self.Outer_Interact_Icon`) true false)
    (`KismetSystemLibrary.PrintString` "Hello")))

(event `self.Outer_Sphere_Collision.OnComponentEndOverlap`
  (params (OverlappedComponent :type "PrimitiveComponent Object Reference") (OtherActor :type "Actor Object Reference") (OtherComp :type "PrimitiveComponent Object Reference") (OtherBodyIndex :type Integer))
  ;[1 1 1] Interaction icon visibility
  (if (== (`GameplayStatics.GetPlayerCharacter` 0) OtherActor)
    (`SceneComponent.SetVisibility` (`self.Outer_Interact_Icon`) false false)))

(event `self.Inner_Sphere_Collision.OnComponentBeginOverlap`
  (params (OverlappedComponent :type "PrimitiveComponent Object Reference") (OtherActor :type "Actor Object Reference") (OtherComp :type "PrimitiveComponent Object Reference") (OtherBodyIndex :type Integer) (bFromSweep :type Boolean) (SweepResult :type "HitResult Structure (by ref)"))
  ;[1 1 1] Interaction icon visibility
  (if (== OtherActor (`GameplayStatics.GetPlayerCharacter` 0))
    (`SceneComponent.SetVisibility` (`self.Inner_Interact_Icon`) true false)
    (`SceneComponent.SetVisibility` (`self.Outer_Interact_Icon`) false false)))

(event `self.Inner_Sphere_Collision.OnComponentEndOverlap`
  (params (OverlappedComponent :type "PrimitiveComponent Object Reference") (OtherActor :type "Actor Object Reference") (OtherComp :type "PrimitiveComponent Object Reference") (OtherBodyIndex :type Integer))
  ;[1 1 1] Interaction icon visibility
  (if (== (`GameplayStatics.GetPlayerCharacter` 0) OtherActor)
    (`SceneComponent.SetVisibility` (`self.Inner_Interact_Icon`) false false)
    (`SceneComponent.SetVisibility` (`self.Outer_Interact_Icon`) true false)))

(event `/Game/Devoir_remi/Moonlighter/Meca/BPI/BPI_Lighting_object.Interaction`
  (params (Interactor :type "/Game/ThirdPerson/Blueprints/BP_ThirdPersonCharacter Object Reference"))
  ;[1 1 1] creation du widget pour inspecter avec les bonnes ref
  (if (`self.Inspect?`)
    (bind _returnvalue (`|SpawnActorFromClass` "/Game/Devoir_remi/Moonlighter/Meca/BP/inspectable/BP_inspectable.BP_inspectable_C" (`KismetMathLibrary.MakeTransform` (300.0 0.0 0.0)) "Undefined" "MultiplyWithRoot" null null))
    (`KismetSystemLibrary.PrintString` "Hello")
    (`/Game/Devoir_remi/Moonlighter/Meca/BP/inspectable/BP_inspectable.Set_Inspect_Rotation` _returnvalue (`self.Item_inspection_rotation`))
    (`/Game/Devoir_remi/Moonlighter/Meca/BP/inspectable/BP_inspectable.Set_inspect_Scale` _returnvalue (`self.Item_inspection_Scale`))
    (message `/Game/Devoir_remi/Moonlighter/Meca/BPI/BPI_Lighting_object.Inspection` _returnvalue Interactor (`StaticMeshComponent.StaticMesh` (`self.Static_Mesh`)) (`self.Item_name`) (`self.Item_description`))))

(fn `UserConstructionScript`
  (bind _outer_sphere_collision (`self.Outer_Sphere_Collision`))
  (bind _inner_sphere_collision (`self.Inner_Sphere_Collision`))
  (bind _static_mesh (`self.Static_Mesh`))
  (`parent.UserConstructionScript`)
  (`|ExecutionSequence`
    (:`then_0`
      ;[1 1 1] Setting Sphère collision radius
      (`SphereComponent.SetSphereRadius` (`self.Inner_Sphere_Collision`) (`self.Inner_Sphere_Radius`) true)
      (`SphereComponent.SetSphereRadius` (`self.Outer_Sphere_Collision`) (`self.Outer_Sphere_Radius`) true))
    (:`then_1`
      ;[1 1 1] set Mesh
      (`StaticMeshComponent.SetStaticMesh` (`self.Static_Mesh`) (`self.Item_Mesh`))
      ;[1 1 1] set scale
      (`SceneComponent.K2_SetWorldTransform` _static_mesh (`KismetMathLibrary.MakeTransform` (`SceneComponent.K2_GetComponentLocation` _static_mesh) (`SceneComponent.K2_GetComponentRotation` _static_mesh) (`self.Item_scale`)) false false))
    (:`then_2`
      ;[1 1 1] voir les radius pour du debbug
      (if (`self.Debbugin?`)
        (`SceneComponent.SetVisibility` _inner_sphere_collision true false)
        (`SceneComponent.SetVisibility` _outer_sphere_collision true false)
        (else
          (`SceneComponent.SetVisibility` _inner_sphere_collision false false)
          (`SceneComponent.SetVisibility` _outer_sphere_collision false false))))))